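; Third-person player character Blueprint handling movement, mouse look, sprint, crouch and weapon aiming.
; Boolean flags gate the states: Shift raises walk speed and blocks WASD, leaving a separate Sprint axis to move forward unless Ctrl is held.
; Right mouse plays standing or crouched weapon-hold montages, which Tick stops while sprinting.
; As wired, Ctrl calls Crouch only when interrupting a sprint, and always uncrouches on release.
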(event EventBeginPlay
  (Input|EnableInput (Game|GetPlayerController 0))
  (Variables|Default|SetCanReceivedInput true)
  (Variables|Default|SetSprintButtonPressed false))

(event EventTick
  (params (DeltaSeconds :type Float%20%28single-precision%29))
  (if (Variables|Default|GetSprintButtonPressed)
    (Animation|StopAnimMontage "/Game/TPS/M_TPS_WeaponHoldCrouch.M_TPS_WeaponHoldCrouch")
    (Animation|StopAnimMontage "/Game/TPS/M_TPS_WeaponHoldNormal.M_TPS_WeaponHoldNormal")))

(event Input|AxisEvents|InputAxisTurn
  (params (AxisValue :type Float%20%28single-precision%29))
  ;[1 1 1] MouseControl
  (Pawn|Input|AddControllerYawInput AxisValue))

(event Input|AxisEvents|InputAxisLookUp
  (params (AxisValue :type Float%20%28single-precision%29))
  ;[1 1 1] MouseControl
  (Pawn|Input|AddControllerPitchInput AxisValue))

(event Input|AxisEvents|InputAxisMoveRight
  (params (AxisValue :type Float%20%28single-precision%29))
  ;[1 1 1] WASD
  (if (Variables|Default|GetCanReceivedInput)
    (Pawn|Input|AddMovementInput (Math|Vector|GetRightVector (Math|Rotator|MakeRotator 0.0 0.0 (.Yaw (Math|Rotator|BreakRotator (Pawn|GetControlRotation :!class /Script/Engine.Pawn))))) (.Y (Math|Vector|BreakVector (Math|Vector|Normalize (Math|Vector|MakeVector (stale Input|AxisEvents|InputAxisMoveForward AxisValue) AxisValue 0.0)))) false)))

(event Input|AxisEvents|InputAxisMoveForward
  (params (AxisValue :type Float%20%28single-precision%29))
  ;[1 1 1] WASD
  (if (Variables|Default|GetCanReceivedInput)
    (Pawn|Input|AddMovementInput (Math|Vector|GetForwardVector (Math|Rotator|MakeRotator 0.0 0.0 (.Yaw (Math|Rotator|BreakRotator (Pawn|GetControlRotation :!class /Script/Engine.Pawn))))) (.X (Math|Vector|BreakVector (Math|Vector|Normalize (Math|Vector|MakeVector AxisValue (stale Input|AxisEvents|InputAxisMoveRight AxisValue) 0.0)))) false)))

(event Input|AxisEvents|InputAxisSprint
  (params (AxisValue :type Float%20%28single-precision%29))
  ;[1 1 1] Sprint
  (if (not (Variables|Default|GetCrouchButtonPressed))
    (Pawn|Input|AddMovementInput (Math|Vector|GetForwardVector (Math|Rotator|MakeRotator 0.0 0.0 (.Yaw (Math|Rotator|BreakRotator (Pawn|GetControlRotation :!class /Script/Engine.Pawn))))) AxisValue false)))

(event Input|KeyboardEvents|LeftCtrl
  (params (Key :type Key%20Structure))
  (bind _mesh (Variables|Character|GetMesh))
  (bind _rightmousebuttonpressed (Variables|Default|GetRightMouseButtonPressed))
  ;[1 1 1] Crouch
  (:Pressed
    (Variables|Default|SetCrouchButtonPressed true)
    (if (Variables|Default|GetSprintButtonPressed)
      (Variables|Default|SetSprintButtonPressed false)
      (Variables|Default|SetCanReceivedInput true)
      (Character|Crouch)
      (if _rightmousebuttonpressed
        (Animation|Montage|PlayMontage _mesh "/Game/TPS/M_TPS_WeaponHoldCrouch.M_TPS_WeaponHoldCrouch"))))
  (:Released
    (Variables|Default|SetCrouchButtonPressed false)
    (Character|UnCrouch)
    (if _rightmousebuttonpressed
      (Animation|Montage|PlayMontage _mesh "/Game/TPS/M_TPS_WeaponHoldNormal.M_TPS_WeaponHoldNormal"))))

(event Input|MouseEvents|RightMouseButton
  (params (Key :type Key%20Structure))
  (bind _mesh (Variables|Character|GetMesh))
  ;[1 1 1] Aiming( Normal/Crouching)
  (:Pressed
    (if (not (Variables|Default|GetSprintButtonPressed))
      (Variables|Default|SetRightMouseButtonPressed true)
      (if (Variables|Default|GetCrouchButtonPressed)
        (Animation|Montage|PlayMontage _mesh "/Game/TPS/M_TPS_WeaponHoldCrouch.M_TPS_WeaponHoldCrouch")
        (else
          (Animation|Montage|PlayMontage _mesh "/Game/TPS/M_TPS_WeaponHoldNormal.M_TPS_WeaponHoldNormal")))))
  (:Released
    (Variables|Default|SetRightMouseButtonPressed false)
    (if (Variables|Default|GetCrouchButtonPressed)
      (Animation|StopAnimMontage "/Game/TPS/M_TPS_WeaponHoldCrouch.M_TPS_WeaponHoldCrouch")
      (else
        (Animation|StopAnimMontage "/Game/TPS/M_TPS_WeaponHoldNormal.M_TPS_WeaponHoldNormal")))))

(event Input|KeyboardEvents|LeftShift
  (params (Key :type Key%20Structure))
  ;[1 1 1] Sprint
  (:Pressed
    (if (not (Variables|Default|GetCrouchButtonPressed))
      (Variables|Default|SetCanReceivedInput false)
      (Variables|Default|SetSprintButtonPressed true)
      (Variables|/Script/Engine.CharacterMovementComponent|SetMaxWalkSpeed (Variables|Character|GetCharacterMovement) 2e+03)))
  (:Released
    (Variables|Default|SetCanReceivedInput true)
    (Variables|Default|SetSprintButtonPressed false)
    (Variables|/Script/Engine.CharacterMovementComponent|SetMaxWalkSpeed (Variables|Character|GetCharacterMovement) 6e+02)))

(fn ConstructionScript)